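; BP_PotCol is a cauldron that asks for a randomly colored potion, shown by the material on its Cylinder.
; On BeginPlay it picks one of eight colors as WantedColor.
; When a BP_GrabActor overlaps the Capsule, a matching PotionColor plays a success sound and rerolls the color, while a mismatch only logs.
; Either way, the potion teleports back to its reset position.
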(event OnComponentBeginOverlap(Capsule)
  (params (OverlappedComponent :type Primitive%20Component%20Object%20Reference) (OtherActor :type Actor%20Object%20Reference) (OtherComp :type Primitive%20Component%20Object%20Reference) (OtherBodyIndex :type Integer) (bFromSweep :type Boolean) (SweepResult :type Hit%20Result%20Structure%20%28by%20ref%29))
  ;[1 1 1] Check the color of the potion that enters the pot and show as a debug string
  (bind _asbp_grab_actor (Utilities|Casting|CastToBP_GrabActor OtherActor))
  (if (== (Variables|Default|GetWantedColor) (Variables|/Game/Blueprints/BP_GrabActor.BP_GrabActor_C|GetPotionColor _asbp_grab_actor))
    (Audio|PlaySound2D "/Game/Sounds/Correct_Cue.Correct_Cue" 0.1 1.0 0.0 0 0)
    (CallFunction|RandomColorandApply)
    (else
      (Development|PrintString "No es el mismo color" false)))
  (Transformation|SetActorLocation _asbp_grab_actor (Variables|/Game/Blueprints/BP_GrabActor.BP_GrabActor_C|GetResetPos _asbp_grab_actor) false true))

(event OnComponentEndOverlap(Capsule)
  (params (OverlappedComponent :type Primitive%20Component%20Object%20Reference) (OtherActor :type Actor%20Object%20Reference) (OtherComp :type Primitive%20Component%20Object%20Reference) (OtherBodyIndex :type Integer))
  ;[1 1 1] Check if the potion leaves the pot and say it
  (Utilities|Casting|CastToBP_GrabActor OtherActor)
  (Development|PrintString "Pocion fuera del caldero" false))

(event EventBeginPlay
  (CallFunction|RandomColorandApply))

(event Collision|EventActorBeginOverlap
  (params (OtherActor :type Actor%20Object%20Reference)))

(event EventTick
  (params (DeltaSeconds :type Float%20%28single-precision%29)))

(fn ConstructionScript)

(fn RandomColorandApply
  (bind _cylinder (Variables|Default|GetCylinder))
  (bind _output_get (Variables|Default|SetWantedColor (Math|Random|RandomInteger 8)))
  (switch int _output_get
    (:0
      (Rendering|Material|SetMaterial _cylinder 0 "/Game/Materials/M_Black.M_Black"))
    (:1
      (Rendering|Material|SetMaterial _cylinder 0 "/Game/Materials/M_Red.M_Red"))
    (:2
      (Rendering|Material|SetMaterial _cylinder 0 "/Game/Materials/M_Blue.M_Blue"))
    (:3
      (Rendering|Material|SetMaterial _cylinder 0 "/Game/Materials/M_Green.M_Green"))
    (:4
      (Rendering|Material|SetMaterial _cylinder 0 "/Game/Materials/M_Orange.M_Orange"))
    (:5
      (Rendering|Material|SetMaterial _cylinder 0 "/Game/Materials/M_Pink.M_Pink"))
    (:6
      (Rendering|Material|SetMaterial _cylinder 0 "/Game/Materials/M_Yellow.M_Yellow"))
    (:7
      (Rendering|Material|SetMaterial _cylinder 0 "/Game/Materials/M_White.M_White"))))