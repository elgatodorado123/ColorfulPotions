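; BP_GrabActor is a potion actor that takes on one of eight colours based on its PotionColor value.
; On BeginPlay it caches the Potion component's world location in ResetPos, then switches on PotionColor to assign the matching material to element 1.
; No grab or reset logic appears in its graphs, and the overlap, tick and construction script are empty.
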(event EventBeginPlay
  (bind _potion (Variables|Default|GetPotion))
  ;[1 1 1] Check Color and change material
  (Variables|Default|SetResetPos (Transformation|GetWorldLocation (Variables|Default|GetPotion)))
  (switch int (Variables|Default|GetPotionColor)
    (:0
      (Rendering|Material|SetMaterial _potion 1 "/Game/Materials/M_Black.M_Black"))
    (:1
      (Rendering|Material|SetMaterial _potion 1 "/Game/Materials/M_Red.M_Red"))
    (:2
      (Rendering|Material|SetMaterial _potion 1 "/Game/Materials/M_Blue.M_Blue"))
    (:3
      (Rendering|Material|SetMaterial _potion 1 "/Game/Materials/M_Green.M_Green"))
    (:4
      (Rendering|Material|SetMaterial _potion 1 "/Game/Materials/M_Orange.M_Orange"))
    (:5
      (Rendering|Material|SetMaterial _potion 1 "/Game/Materials/M_Pink.M_Pink"))
    (:6
      (Rendering|Material|SetMaterial _potion 1 "/Game/Materials/M_Yellow.M_Yellow"))
    (:7
      (Rendering|Material|SetMaterial _potion 1 "/Game/Materials/M_White.M_White"))))

(event Collision|EventActorBeginOverlap
  (params (OtherActor :type Actor%20Object%20Reference)))

(event EventTick
  (params (DeltaSeconds :type Float%20%28single-precision%29)))

(fn ConstructionScript)